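; HeartTowerBP is a player-controlled turret that aims from input axes and fires a debug trace.
; Each tick, axis input yaws the turret's mid section and rolls the gun, with roll clamped between 0 and 50 degrees.
; Left mouse runs a visibility multi-line trace from Arrow1, using the scaled Arrow1-minus-Arrow2 vector directly as the end point.
; The trace only draws debug lines; its hits are unused.
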(event EventBeginPlay)

(event Collision|EventActorBeginOverlap
  (params (OtherActor :type Actor%20Object%20Reference)))

(event EventTick
  (params (DeltaSeconds :type Float%20%28single-precision%29))
  (bind _returnvalue (Class|Actor|GetInputAxisKeyValue))
  (bind _flame_turret_long_1_gun (Variables|Default|GetFlame_Turret_Long_1_Gun))
  (bind _flame_turret_long_1_mid (Variables|Default|GetFlame_Turret_Long_1_Mid))
  (bind _returnvalue_2 (* _returnvalue -1.0))
  (bind _relativerotation (Variables|/Script/Engine.SceneComponent|GetRelativeRotation _flame_turret_long_1_gun))
  (bind _returnvalue_3 (Math|Rotator|MakeRotator _returnvalue_2 0.0 0.0))
  (bind _returnvalue_4 (Math|Rotator|CombineRotators _relativerotation _returnvalue_3))
  (Transformation|SetRelativeRotation _flame_turret_long_1_mid (Math|Rotator|CombineRotators (Variables|/Script/Engine.SceneComponent|GetRelativeRotation _flame_turret_long_1_mid) (Math|Rotator|MakeRotator 0.0 0.0 (Class|Actor|GetInputAxisKeyValue))) false false)
  (bind _output_get (Variables|Default|SetReturn%20Value%20X%20%28Roll%29 (.roll _returnvalue_4)))
  (if (>= (.roll _returnvalue_4) 5e+01)
    (Variables|Default|SetReturn%20Value%20X%20%28Roll%29 5e+01))
  (if (<= _output_get 0.0)
    (Variables|Default|SetReturn%20Value%20X%20%28Roll%29 0.0))
  (Transformation|SetRelativeRotation _flame_turret_long_1_gun (Math|Rotator|MakeRotator (Variables|Default|GetReturn%20Value%20X%20%28Roll%29) (.pitch _returnvalue_4) (.yaw _returnvalue_4)) false false))

(event Input|MouseEvents|LeftMouseButton
  (params (Key :type Key%20Structure :default "None"))
  (bind _arrow1 (Variables|Default|GetArrow1))
  (bind _returnvalue (Transformation|GetWorldLocation _arrow1))
  (:Pressed
    (Collision|MultiLineTraceByChannel _returnvalue (* (- _returnvalue (Transformation|GetWorldLocation (Variables|Default|GetArrow2))) 1e+02) "TraceTypeQuery1" false 0 "ForDuration")))

(fn ConstructionScript)