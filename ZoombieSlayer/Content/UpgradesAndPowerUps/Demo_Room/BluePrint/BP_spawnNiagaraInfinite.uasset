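; Demo-room actor that displays a chosen Niagara effect and can replay it on a repeating interval.
; The construction script assigns the configured system asset to the Niagara component.
; When Reset is enabled, BeginPlay starts a looping timer with a configurable interval and reassigns the asset; each timer tick calls Respawn, which resets the Niagara system.
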(event Custom|Respawn
  (Niagara|ResetSystem (Variables|Default|GetNiagara)))

(event EventBeginPlay
  (if (Variables|Default|Getreset)
    (Utilities|Time|SetTimerbyFunctionName 0 "respawn" (Variables|Default|GetTime) true)
    (Class|NiagaraComponent|SetAsset (Variables|Default|GetNiagara) (Variables|Default|GetIn%20Asset) true)))

(event Collision|EventActorBeginOverlap
  (params (OtherActor :type Actor%20Object%20Reference)))

(event EventTick
  (params (DeltaSeconds :type Float%20%28single-precision%29)))

(fn ConstructionScript
  (if true
    _
    (else
      _))
  (Class|NiagaraComponent|SetAsset (Variables|Default|GetNiagara) (Variables|Default|GetIn%20Asset) true))